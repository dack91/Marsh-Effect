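; Toxic flood puzzle actor: the player must press three pump buttons to drain a deadly flood.
; Button triggers track range and briefly show help text, and pressing E marks that button pressed.
; Once all three are pressed, a timeline lowers the flood, then destroys it.
; Touching the flood drains health on a looping timer for two seconds, then respawns the player at full health and resets the buttons.
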(event `self.ReceiveBeginPlay`
  ;[1 1 1] Get player character
  (bind _asmy_player (cast `/Game/Blueprints/MyPlayer` (`GameplayStatics.GetPlayerCharacter` 0)))
  (set `self.Player1` _asmy_player)
  ;[1 1 1] Enable Player Input
  (`self.EnableInput` (`GameplayStatics.GetPlayerController` 0))
  ;[1 1 1] Inintialize Puzzle Help UI
  (bind _returnvalue (`|CreateWidget` "/Game/Blueprints/UI/HelpTextUI_BP.HelpTextUI_BP_C"))
  (bind _output_get (set `self.floodUI` _returnvalue))
  (`UserWidget.AddToViewport` _output_get 0)
  ;[1 1 1] Set help text for pump controls
  (set `/Game/Blueprints/UI/HelpTextUI_BP.helpText` (`self.FloodButtonText`) (`self.floodUI`)))

(event `self.ToxicFlood.OnComponentBeginOverlap`
  (params (OverlappedComponent :type "PrimitiveComponent Object Reference") (OtherActor :type "Actor Object Reference") (OtherComp :type "PrimitiveComponent Object Reference") (OtherBodyIndex :type Integer) (bFromSweep :type Boolean) (SweepResult :type "HitResult Structure (by ref)"))
  ;[1 1 1] Player dies on contact with flood
  (cast `/Game/Blueprints/MyPlayer` OtherActor)
  (`AudioComponent.Play` (`self.splashSound`) 0.0)
  (`AudioComponent.Play` (`self.DeathSound`) 0.0)
  (bind _returnvalue (`KismetSystemLibrary.K2_SetTimer` null "damageHealth" 0.2 true))
  (`KismetSystemLibrary.Delay` 2.0)
  (`KismetSystemLibrary.K2_ClearAndInvalidateTimerHandle` _returnvalue)
  (`self.K2_SetActorLocation` (`GameplayStatics.GetPlayerPawn` 0) (`/Game/Blueprints/MyPlayer.spawnLocation` (`self.Player1`)) false false) ; Reset Position
  (set `/Game/Blueprints/MyPlayer.health` 1.0 (`self.Player1`))
  ;[1 1 1] Reset pump control buttons
  (set `self.button1IsPressed` false)
  (set `self.button2IsPressed` false)
  (set `self.button3IsPressed` false))

(event `self.Button1Trigger.OnComponentBeginOverlap`
  (params (OverlappedComponent :type "PrimitiveComponent Object Reference") (OtherActor :type "Actor Object Reference") (OtherComp :type "PrimitiveComponent Object Reference") (OtherBodyIndex :type Integer) (bFromSweep :type Boolean) (SweepResult :type "HitResult Structure (by ref)"))
  (bind _floodui (`self.floodUI`))
  ;[1 1 1] Monitor Player in Range of pump buttons
  (set `self.button1IsInRange` true)
  ;[1 1 1] Toggle Lift Help UI
  (set `/Game/Blueprints/UI/HelpTextUI_BP.helpTextVisibility` "Visible" _floodui :!label _label)
  (`KismetSystemLibrary.Delay` 3.0)
  (set `/Game/Blueprints/UI/HelpTextUI_BP.helpTextVisibility` "Hidden" _floodui))

(event `self.Button2Trigger.OnComponentBeginOverlap`
  (params (OverlappedComponent :type "PrimitiveComponent Object Reference") (OtherActor :type "Actor Object Reference") (OtherComp :type "PrimitiveComponent Object Reference") (OtherBodyIndex :type Integer) (bFromSweep :type Boolean) (SweepResult :type "HitResult Structure (by ref)"))
  ;[1 1 1] Monitor Player in Range of pump buttons
  (set `self.button2IsInRange` true)
  (goto _label))

(event `self.Button3Trigger.OnComponentBeginOverlap`
  (params (OverlappedComponent :type "PrimitiveComponent Object Reference") (OtherActor :type "Actor Object Reference") (OtherComp :type "PrimitiveComponent Object Reference") (OtherBodyIndex :type Integer) (bFromSweep :type Boolean) (SweepResult :type "HitResult Structure (by ref)"))
  ;[1 1 1] Monitor Player in Range of pump buttons
  (set `self.button3IsInRange` true)
  (goto _label))

(event `Key|E`
  (params (Key :type "Key Structure" :default "AnyKey"))
  (bind _location (.location (`SceneComponent.GetRelativeTransform` (`self.ToxicFlood`))))
  (:`Pressed`
    ;[1 1 1] Push all three pump buttons
    (if (`self.button1IsInRange`)
      (set `self.button1IsPressed` true)
      ;[1 1 1] Drain Flood
      (`self.isPumpActive` :!label _label_2)
      (`AudioComponent.Play` (`self.buttonSound`) 0.0)
      (if (`self.pumpActive`)
        (`AudioComponent.Play` (`self.pumpMotorSound`) 0.0)
        (bind (_direction _driver) (`Timeline|FloodDrainTimeline`)
          (:`Update`
            (`SceneComponent.K2_SetRelativeLocation` (`self.ToxicFlood`) (`KismetMathLibrary.VLerp` _location (+ _location (0.0 0.0 -0.68)) _driver) false false))
          (:`Finished`
            (`ActorComponent.K2_DestroyComponent` (`self.ToxicFlood`))
            (`AudioComponent.Stop` (`self.pumpMotorSound`)))))
      (elif (`self.button2IsInRange`)
        (set `self.button2IsPressed` true)
        (goto _label_2)
        (elif (`self.button3IsInRange`)
          (set `self.button3IsPressed` true)
          (goto _label_2))))))

(event `self.Button1Trigger.OnComponentEndOverlap`
  (params (OverlappedComponent :type "PrimitiveComponent Object Reference") (OtherActor :type "Actor Object Reference") (OtherComp :type "PrimitiveComponent Object Reference") (OtherBodyIndex :type Integer))
  ;[1 1 1] Monitor Player in Range of pump buttons
  (set `self.button1IsInRange` false)
  ;[1 1 1] Toggle Lift Help UI
  (set `/Game/Blueprints/UI/HelpTextUI_BP.helpTextVisibility` "Hidden" (`self.floodUI`) :!label _label_3))

(event `self.Button2Trigger.OnComponentEndOverlap`
  (params (OverlappedComponent :type "PrimitiveComponent Object Reference") (OtherActor :type "Actor Object Reference") (OtherComp :type "PrimitiveComponent Object Reference") (OtherBodyIndex :type Integer))
  ;[1 1 1] Monitor Player in Range of pump buttons
  (set `self.button2IsInRange` false)
  (goto _label_3))

(event `self.Button3Trigger.OnComponentEndOverlap`
  (params (OverlappedComponent :type "PrimitiveComponent Object Reference") (OtherActor :type "Actor Object Reference") (OtherComp :type "PrimitiveComponent Object Reference") (OtherBodyIndex :type Integer))
  ;[1 1 1] Monitor Player in Range of pump buttons
  (set `self.button3IsInRange` false)
  (goto _label_3))

(fn `damageHealth`
  (set `/Game/Blueprints/MyPlayer.health` (- (`/Game/Blueprints/MyPlayer.health` (`self.Player1`)) 0.1) (`self.Player1`)))

(fn `isPumpActive`
  (returns (isActive :type Boolean))
  (if (`self.button1IsPressed`)
    (if (`self.button2IsPressed`)
      (if (`self.button3IsPressed`)
        (set `self.pumpActive` true) ; All Buttons Pressed
        (else
          (set `self.pumpActive` false :!label _label) ; One or more buttons not pressed
        ))
      (else
        (goto _label)))
    (else
      (goto _label)))
  (return (`self.pumpActive`)))

(fn `UserConstructionScript`)
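; An oxygen terminal actor that the player uses with the F key to lower their ReductionBonus stat.
; It enables input from player controller 0 on BeginPlay and flags overlap with any actor.
; While flagged, each press finds the first MyPlayer actor and subtracts a fraction of its BlueMineral from ReductionBonus, without consuming the mineral.
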(event `self.ReceiveBeginPlay`
  ;[1 1 1] get input from player my dudes
  (`self.EnableInput` (`GameplayStatics.GetPlayerController` 0)))

(event `self.ReceiveActorBeginOverlap`
  (params (OtherActor :type "Actor Object Reference"))
  (set `self.playerTouchingMe` true))

(event `self.ReceiveActorEndOverlap`
  (params (OtherActor :type "Actor Object Reference"))
  (set `self.playerTouchingMe` false))

(event `Key|F`
  (params (Key :type "Key Structure" :default "AnyKey"))
  (:`Pressed`
    (if (`self.playerTouchingMe`)
      (bind _outactors (`GameplayStatics.GetAllActorsOfClass` "/Game/Blueprints/MyPlayer.MyPlayer_C"))
      (bind _item (`KismetArrayLibrary.Array_Get` _outactors))
      (set `/Game/Blueprints/MyPlayer.ReductionBonus` (- (`/Game/Blueprints/MyPlayer.ReductionBonus` _item) (* (`/Game/Blueprints/MyPlayer.blueMineral` _item) 0.05)) _item))))

(fn `UserConstructionScript`)
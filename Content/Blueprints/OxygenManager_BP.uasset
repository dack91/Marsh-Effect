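; Oxygen manager actor that drains or refills the player's oxygen and health as they move between indoors and outdoors.
; Overlaps by the player or a HoverCar flip an outside flag, which swaps looping depletion and replenish timers.
; Depletion scales with the player's reduction bonus and damages health below half oxygen.
; Empty oxygen returns the player to spawn, moves the first HoverCar to world origin and restores stats.
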(event `self.ReceiveBeginPlay`
  ;[1 1 1] Get Reference to Player
  (bind _asmy_player (cast `/Game/Blueprints/MyPlayer` (`GameplayStatics.GetPlayerCharacter` 0)))
  (set `self.Player1` _asmy_player))

(event `self.ReceiveActorBeginOverlap`
  (params (OtherActor :type "Actor Object Reference"))
  ;[1 1 1] Toggle Inside/Outside game state
  (`|ExecutionSequence`
    (:`then_0`
      (cast `/Game/Blueprints/MyPlayer` OtherActor))
    (:`then_1`
      (cast `/Game/FirstPersonBP/Blueprints/HoverCar` OtherActor)))
  (`self.TogglePlayerIndoorOutdoor`))

(event `PlayerOutside`
  ;[1 1 1] Player inside and outside oxygen behavoir
  (bind _returnvalue (`KismetSystemLibrary.K2_SetTimer` null "OxygenDamage" (`self.OxygenReplenishRate`) true))
  (`KismetSystemLibrary.K2_ClearAndInvalidateTimerHandle` (stale `PlayerInside` _returnvalue)))

(event `PlayerInside`
  ;[1 1 1] Player inside and outside oxygen behavoir
  (`KismetSystemLibrary.K2_ClearAndInvalidateTimerHandle` (stale `PlayerOutside` _returnvalue))
  (bind _returnvalue (`KismetSystemLibrary.K2_SetTimer` null "OxygenReplenish" (`self.OxygenReplenishRate`) true)))

(fn `OxygenDamage`
  (bind _player1 (`self.Player1`))
  (bind _player1_2 (`self.Player1`))
  ;[1 1 1] Deplete Oxygen
  (set `/Game/Blueprints/MyPlayer.oxygenTank` (- (`/Game/Blueprints/MyPlayer.oxygenTank` (`self.Player1`)) (* 0.005 (`/Game/Blueprints/MyPlayer.ReductionBonus` (`self.Player1`)))) (`self.Player1`))
  (if (> (`/Game/Blueprints/MyPlayer.oxygenTank` (`self.Player1`)) 0.0)
    (if (< (`/Game/Blueprints/MyPlayer.oxygenTank` (`self.Player1`)) 0.5)
      ;[1 1 1] Damage Player Health
      (set `/Game/Blueprints/MyPlayer.health` (- (`/Game/Blueprints/MyPlayer.health` _player1_2) 0.02) _player1_2))
    (else
      ;[1 1 1] Oxygen Out, Reset Player
      (`AudioComponent.Play` (`self.dieReturnToHangerSound`) 0.0) ; Reset SFX
      (`self.K2_SetActorLocation` (`GameplayStatics.GetPlayerPawn` 0) (`/Game/Blueprints/MyPlayer.spawnLocation` (`self.Player1`)) false false) ; Reset Position
      (bind _outactors (`GameplayStatics.GetAllActorsOfClass` "/Game/FirstPersonBP/Blueprints/HoverCar.HoverCar_C"))
      (`self.K2_SetActorLocation` (`KismetArrayLibrary.Array_Get` _outactors) (0.0 0.0 0.0) false false) ; Reset Position
      (set `self.playerIsOutside` false) ; Reset Player State
      (set `/Game/Blueprints/MyPlayer.oxygenTank` (`/Game/Blueprints/MyPlayer.MAX_OXYGEN` _player1) _player1)
      (set `/Game/Blueprints/MyPlayer.health` 1.0 (`self.Player1`))
      (`self.PlayerInside`) ; Reset Event
    )))

(fn `OxygenReplenish`
  (bind _player1 (`self.Player1`))
  (bind _player1_2 (`self.Player1`))
  (bind _player1_3 (`self.Player1`))
  (if (< (`/Game/Blueprints/MyPlayer.oxygenTank` _player1) (`/Game/Blueprints/MyPlayer.MAX_OXYGEN` _player1))
    ;[1 1 1] Fill Tank
    (set `/Game/Blueprints/MyPlayer.oxygenTank` (+ (`/Game/Blueprints/MyPlayer.oxygenTank` _player1_2) 0.05) _player1_2)
    (if (not (>= (`/Game/Blueprints/MyPlayer.health` (`self.Player1`)) 1.0))
      ;[1 1 1] Heal Player
      (set `/Game/Blueprints/MyPlayer.health` (+ (`/Game/Blueprints/MyPlayer.health` _player1_3) 0.02) _player1_3))))

(fn `TogglePlayerIndoorOutdoor`
  (set `self.playerIsOutside` (not (`self.playerIsOutside`)))
  (if (`self.playerIsOutside`)
    (`self.PlayerOutside`)
    (else
      (`self.PlayerInside`))))

(fn `UserConstructionScript`)
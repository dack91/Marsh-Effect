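; Elevator actor that moves the Ship2 platform between Levels 1, 2 and 4 on player key presses.
; E rides up one stop or, off the lift, calls it to the player's level; R rides down one stop.
; Overlap triggers set player flags without filtering the overlapping actor, while booleans track the lift's stop.
; Timelines lerp the platform's relative location, some reversed for calls, with CanMove blocking input during travel.
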(event `self.ReceiveBeginPlay`
  ;[1 1 1] Enable Player Input
  (`self.EnableInput` (`GameplayStatics.GetPlayerController` 0)))

(event `Key|E`
  (params (Key :type "Key Structure" :default "AnyKey"))
  ;[1 1 1] Elevator Movement
  (:`Pressed`
    ;;[1 0.879 0] Ride Lift Up
    (if (`self.isPlayerOnLift`)
      (if (`self.canMove`)
        (`|ExecutionSequence`
          (:`then_0`
            (if (`self.isPlayerAtLevel1`)
              ;;;[0 1 0.4029] To Level 2
              (`|ExecutionSequence`
                (:`then_0`
                  (set `self.isLiftAtLevel2` true)
                  (set `self.isLiftAtLevel1` false))
                (:`then_1`
                  (set `self.canMove` false)
                  (bind (_direction _driver) (`Timeline|Timeline_Lift1` :!via `PlayFromStart` :!label _label)
                    (:`Update`
                      (`SceneComponent.K2_SetRelativeLocation` (`self.ship2_elevator_platform`) (`KismetMathLibrary.VLerp` (`self.Level1`) (`self.Level2`) _driver) false false))
                    (:`Finished`
                      (set `self.canMove` true)))))))
          (:`then_1`
            (if (`self.isPlayerAtLevel2`)
              ;;;[0 0.04925 1] To Level 4
              (`|ExecutionSequence`
                (:`then_0`
                  (set `self.isLiftAtLevel2` false)
                  (set `self.isLiftAtLevel4` true))
                (:`then_1`
                  (set `self.canMove` false)
                  (bind (_direction_2 _driver_2) (`Timeline|Timeline_Lift2` :!via `PlayFromStart`)
                    (:`Update`
                      (`SceneComponent.K2_SetRelativeLocation` (`self.ship2_elevator_platform`) (`KismetMathLibrary.VLerp` (`self.Level2`) (`self.Level4`) _driver_2) false false))
                    (:`Finished`
                      (set `self.canMove` true)))))))))
      (else
        ;;[1 0.03562 0] Call Lift to Player Level
        (if (`self.isPlayerAtLevel1`)
          (if (`self.canMove`)
            ;;;[1 0.5061 0] Call to Level 1
            (if (`self.isLiftAtLevel2`)
              (`|ExecutionSequence`
                (:`then_0`
                  (set `self.canMove` false))
                (:`then_1`
                  (set `self.isLiftAtLevel2` false)
                  (set `self.isLiftAtLevel1` true)
                  (goto _label :!via `ReverseFromEnd`)))
              (elif (`self.isLiftAtLevel4`)
                (`|ExecutionSequence`
                  (:`then_0`
                    (set `self.canMove` false))
                  (:`then_1`
                    (set `self.isLiftAtLevel4` false)
                    (set `self.isLiftAtLevel1` true)
                    (bind (_direction_3 _driver_3) (`Timeline|Timeline_Lift5` :!via `PlayFromStart` :!label _label_2)
                      (:`Update`
                        (`SceneComponent.K2_SetRelativeLocation` (`self.ship2_elevator_platform`) (`KismetMathLibrary.VLerp` (`self.Level4`) (`self.Level1`) _driver_3) false false))
                      (:`Finished`
                        (set `self.canMove` true))))))))
          (elif (`self.isPlayerAtLevel2`)
            (if (`self.canMove`)
              ;;;[0 1 0.6226] Call to Level 2
              (if (`self.isLiftAtLevel1`)
                (`|ExecutionSequence`
                  (:`then_0`
                    (set `self.canMove` false))
                  (:`then_1`
                    (set `self.isLiftAtLevel1` false)
                    (set `self.isLiftAtLevel2` true)
                    (goto _label :!via `PlayFromStart`)))
                (elif (`self.isLiftAtLevel4`)
                  (`|ExecutionSequence`
                    (:`then_0`
                      (set `self.canMove` false))
                    (:`then_1`
                      (set `self.isLiftAtLevel4` false)
                      (set `self.isLiftAtLevel2` true)
                      ;;[1 0.1598 0.8264] Ride Lift Down
                      ;;;[0 1 0.4029] To Level 2
                      (bind (_direction_4 _driver_4) (`Timeline|Timeline_Lift3` :!via `PlayFromStart` :!label _label_3)
                        (:`Update`
                          (`SceneComponent.K2_SetRelativeLocation` (`self.ship2_elevator_platform`) (`KismetMathLibrary.VLerp` (`self.Level4`) (`self.Level2`) _driver_4) false false))
                        (:`Finished`
                          (set `self.canMove` true))))))))
            (elif (`self.isPlayerAtLevel4`)
              (if (`self.canMove`)
                ;;;[0 0.1456 1] Call to Level 4
                (if (`self.isLiftAtLevel2`)
                  (`|ExecutionSequence`
                    (:`then_0`
                      (set `self.canMove` false))
                    (:`then_1`
                      (set `self.isLiftAtLevel2` false)
                      (set `self.isLiftAtLevel4` true)
                      (goto _label_3 :!via `ReverseFromEnd`)))
                  (elif (`self.isLiftAtLevel1`)
                    (`|ExecutionSequence`
                      (:`then_0`
                        (set `self.canMove` false))
                      (:`then_1`
                        (set `self.isLiftAtLevel1` false)
                        (set `self.isLiftAtLevel4` true)
                        (goto _label_2 :!via `ReverseFromEnd`)))))))))))))

(event `self.LiftTrigger.OnComponentBeginOverlap`
  (params (OverlappedComponent :type "PrimitiveComponent Object Reference") (OtherActor :type "Actor Object Reference") (OtherComp :type "PrimitiveComponent Object Reference") (OtherBodyIndex :type Integer) (bFromSweep :type Boolean) (SweepResult :type "HitResult Structure (by ref)"))
  ;[1 1 1] Trigger Management
  (set `self.isPlayerOnLift` true))

(event `self.LiftTrigger.OnComponentEndOverlap`
  (params (OverlappedComponent :type "PrimitiveComponent Object Reference") (OtherActor :type "Actor Object Reference") (OtherComp :type "PrimitiveComponent Object Reference") (OtherBodyIndex :type Integer))
  ;[1 1 1] Trigger Management
  (set `self.isPlayerOnLift` false))

(event `self.LiftCallLevel1.OnComponentBeginOverlap`
  (params (OverlappedComponent :type "PrimitiveComponent Object Reference") (OtherActor :type "Actor Object Reference") (OtherComp :type "PrimitiveComponent Object Reference") (OtherBodyIndex :type Integer) (bFromSweep :type Boolean) (SweepResult :type "HitResult Structure (by ref)"))
  ;[1 1 1] Trigger Management
  (set `self.isPlayerAtLevel1` true))

(event `self.LiftCallLevel1.OnComponentEndOverlap`
  (params (OverlappedComponent :type "PrimitiveComponent Object Reference") (OtherActor :type "Actor Object Reference") (OtherComp :type "PrimitiveComponent Object Reference") (OtherBodyIndex :type Integer))
  ;[1 1 1] Trigger Management
  (set `self.isPlayerAtLevel1` false))

(event `self.LiftCallLevel2.OnComponentBeginOverlap`
  (params (OverlappedComponent :type "PrimitiveComponent Object Reference") (OtherActor :type "Actor Object Reference") (OtherComp :type "PrimitiveComponent Object Reference") (OtherBodyIndex :type Integer) (bFromSweep :type Boolean) (SweepResult :type "HitResult Structure (by ref)"))
  ;[1 1 1] Trigger Management
  (set `self.isPlayerAtLevel2` true))

(event `self.LiftCallLevel2.OnComponentEndOverlap`
  (params (OverlappedComponent :type "PrimitiveComponent Object Reference") (OtherActor :type "Actor Object Reference") (OtherComp :type "PrimitiveComponent Object Reference") (OtherBodyIndex :type Integer))
  ;[1 1 1] Trigger Management
  (set `self.isPlayerAtLevel2` false))

(event `self.LiftCallLevel4.OnComponentBeginOverlap`
  (params (OverlappedComponent :type "PrimitiveComponent Object Reference") (OtherActor :type "Actor Object Reference") (OtherComp :type "PrimitiveComponent Object Reference") (OtherBodyIndex :type Integer) (bFromSweep :type Boolean) (SweepResult :type "HitResult Structure (by ref)"))
  ;[1 1 1] Trigger Management
  (set `self.isPlayerAtLevel4` true))

(event `self.LiftCallLevel4.OnComponentEndOverlap`
  (params (OverlappedComponent :type "PrimitiveComponent Object Reference") (OtherActor :type "Actor Object Reference") (OtherComp :type "PrimitiveComponent Object Reference") (OtherBodyIndex :type Integer))
  ;[1 1 1] Trigger Management
  (set `self.isPlayerAtLevel4` false))

(event `Key|R`
  (params (Key :type "Key Structure" :default "AnyKey"))
  ;[1 1 1] Elevator Movement
  ;;[1 0.1598 0.8264] Ride Lift Down
  (:`Pressed`
    (if (`self.isPlayerOnLift`)
      (if (`self.canMove`)
        (if (`self.isPlayerAtLevel4`)
          ;;;[0 1 0.4029] To Level 2
          (`|ExecutionSequence`
            (:`then_0`
              (set `self.isLiftAtLevel2` true)
              (set `self.isLiftAtLevel4` false))
            (:`then_1`
              (set `self.canMove` false)
              (goto _label_3 :!via `PlayFromStart`)))
          (elif (`self.isPlayerAtLevel2`)
            ;;;[1 0.4722 0] To Level 1
            (`|ExecutionSequence`
              (:`then_0`
                (set `self.isLiftAtLevel2` false)
                (set `self.isLiftAtLevel1` true))
              (:`then_1`
                (set `self.canMove` false)
                (bind (_direction _driver) (`Timeline|Timeline_Lift4` :!via `PlayFromStart`)
                  (:`Update`
                    (`SceneComponent.K2_SetRelativeLocation` (`self.ship2_elevator_platform`) (`KismetMathLibrary.VLerp` (`self.Level2`) (`self.Level1`) _driver) false false))
                  (:`Finished`
                    (set `self.canMove` true)))))))))))

(fn `UserConstructionScript`)
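; Rock_BP is an interactable rock actor that the player can collect when nearby to give the player blue.
; On BeginPlay it enables input, and each Tick it compares its distance to the player pawn against a threshold, setting CloseEnough and printing a debug string.
; Pressing F while close calls AddBlue on the first MyPlayer found through GetAllActorsOfClass, then destroys the rock.
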(event `self.ReceiveBeginPlay`
  ;[1 1 1] get input from player my dudes
  (`self.EnableInput` (`GameplayStatics.GetPlayerController` 0)))

(event `self.ReceiveTick`
  (params (DeltaSeconds :type "Float (single-precision)"))
  (`/Engine/EditorBlueprintResources/StandardMacros.CompareFloat` (`self.GetDistanceTo` (`GameplayStatics.GetPlayerPawn` 0)) 1000.0
    (:`>`
      (set `self.closeEnough` false))
    (:`<`
      (`KismetSystemLibrary.PrintString` "RIGHT NEXT TO A TING" true true (struct :`G` 0.66 :`B` 1.0 :`A` 1.0) 0.0)
      (set `self.closeEnough` true))))

(event `Key|F` :consume false
  (params (Key :type "Key Structure" :default "AnyKey"))
  (:`Pressed`
    (if (`self.closeEnough`)
      (bind _outactors (`GameplayStatics.GetAllActorsOfClass` "/Game/Blueprints/MyPlayer.MyPlayer_C"))
      (`/Game/Blueprints/MyPlayer.AddBlue` (`KismetArrayLibrary.Array_Get` _outactors))
      (`self.K2_DestroyActor`))))

(fn `UserConstructionScript`)
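; Towers of Hanoi puzzle actor that unlocks the control room door when all five disks reach the third peg.
; Keys 1–3 alternately lift and place disks while the player holds the control fragment inside the solve area, whose overlap also shows help text.
; Integer arrays act as peg stacks for move validation.
; Matching HanoiDisk_BP actors move by world offsets hardcoded to the X axis, so rotating the puzzle requires editing them.
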(event `self.ReceiveBeginPlay`
  ;[1 1 1] Enable Player Input
  (`self.EnableInput` (`GameplayStatics.GetPlayerController` 0))
  ;[1 1 1] Initialize Disks
  (set `self.Disk1` 1)
  (set `self.Disk2` 2)
  (set `self.Disk3` 3)
  (set `self.Disk4` 4)
  (set `self.Disk5` 5)
  ;[1 1 1] Initialize Hanoi Game with all disks on first peg
  (`KismetArrayLibrary.Array_Add` (`self.Peg1`) (`self.Disk5`))
  (`KismetArrayLibrary.Array_Add` (`self.Peg1`) (`self.Disk4`))
  (`KismetArrayLibrary.Array_Add` (`self.Peg1`) (`self.Disk3`))
  (`KismetArrayLibrary.Array_Add` (`self.Peg1`) (`self.Disk2`))
  (`KismetArrayLibrary.Array_Add` (`self.Peg1`) (`self.Disk1`))
  (set `self.NUM_DISKS` (`KismetArrayLibrary.Array_Length` (`self.Peg1`)))
  ;[1 1 1] Initialize list of all disk objects
  (bind _ashanoi_disk_bp (castclass `/Game/Blueprints/HanoiDisk_BP` "/Game/Blueprints/HanoiDisk_BP.HanoiDisk_BP_C"))
  (bind _outactors (`GameplayStatics.GetAllActorsOfClass` _ashanoi_disk_bp))
  (for _array_element _outactors
    (`KismetArrayLibrary.Array_Add` (`self.DiskActors`) _array_element)
    ;[1 1 1] Inintialize Puzzle Help UI
    (bind _returnvalue (`|CreateWidget` "/Game/Blueprints/UI/HelpTextUI_BP.HelpTextUI_BP_C"))
    (bind _output_get (set `self.HanoiUI` _returnvalue))
    (`UserWidget.AddToViewport` _output_get 0)
    ;[1 1 1] Lock Control Room Door
    (bind _asdoor_bp (cast `/Game/Blueprints/Door_BP` (`ChildActorComponent.ChildActor` (`self.Door_BP`))))
    (bind _output_get_2 (set `self.controlRoomDoor` _asdoor_bp))
    (set `/Game/Blueprints/Door_BP.doorCanOpen` false _output_get_2)
    ;[1 1 1] Get player character
    (bind _asmy_player (cast `/Game/Blueprints/MyPlayer` (`GameplayStatics.GetPlayerCharacter` 0)))
    (set `self.Player1` _asmy_player)))

(event `Key|One`
  (params (Key :type "Key Structure" :default "AnyKey"))
  ;[1 1 1] Peg1
  (:`Pressed`
    (if (`/Game/Blueprints/MyPlayer.hasControlFragment` (`self.Player1`))
      (if (`self.playerIsInSolveArea`)
        (bind _pegout (`self.interactWithPeg` (`self.Peg1`) 1))
        (set `self.Peg1` _pegout)))))

(event `Key|P`
  (params (Key :type "Key Structure" :default "AnyKey"))
  ;[1 1 1] Print all Pegs: Debug
  (:`Pressed`
    (`self.printGame`)))

(event `Key|Two`
  (params (Key :type "Key Structure" :default "AnyKey"))
  ;[1 1 1] Peg2
  (:`Pressed`
    (if (`/Game/Blueprints/MyPlayer.hasControlFragment` (`self.Player1`))
      (if (`self.playerIsInSolveArea`)
        (bind _pegout (`self.interactWithPeg` (`self.Peg2`) 2))
        (set `self.Peg2` _pegout)))))

(event `Key|Three`
  (params (Key :type "Key Structure" :default "AnyKey"))
  ;[1 1 1] Peg3
  (:`Pressed`
    (if (`/Game/Blueprints/MyPlayer.hasControlFragment` (`self.Player1`))
      (if (`self.playerIsInSolveArea`)
        (bind _pegout (`self.interactWithPeg` (`self.Peg3`) 3))
        (set `self.Peg3` _pegout)
        (if (`self.isGameOver` (`self.Peg3`))
          ;[1 1 1] Game Won: All disks on final peg
          (`AudioComponent.Play` (`self.SuccessSound`) 0.0)
          ;[1 1 1] Unlock control room door
          (set `/Game/Blueprints/Door_BP.doorCanOpen` true (`self.controlRoomDoor`)))))))

(event `self.PuzzeSolveArea.OnComponentBeginOverlap`
  (params (OverlappedComponent :type "PrimitiveComponent Object Reference") (OtherActor :type "Actor Object Reference") (OtherComp :type "PrimitiveComponent Object Reference") (OtherBodyIndex :type Integer) (bFromSweep :type Boolean) (SweepResult :type "HitResult Structure (by ref)"))
  (bind _player1 (`self.Player1`))
  (bind _hanoiui (`self.HanoiUI`))
  ;[1 1 1] Toggle Player Can Solve Puzzle
  (set `self.playerIsInSolveArea` true)
  ;[1 1 1] Toggle Puzzle Help UI
  (if (and (`/Game/Blueprints/MyPlayer.hasControlFragment` _player1) (`/Game/Blueprints/MyPlayer.hasEngineFragment` _player1) (`/Game/Blueprints/MyPlayer.hasSpeederFragment` _player1) (`/Game/Blueprints/MyPlayer.hasSpeederBoost` _player1) (`/Game/Blueprints/MyPlayer.hasNavigationFragment` _player1))
    (set `/Game/Blueprints/UI/HelpTextUI_BP.helpText` (`self.hanoiHelpText`) _hanoiui)
    (else
      (set `/Game/Blueprints/UI/HelpTextUI_BP.helpText` (`self.controlFragmentErrorText`) (`self.HanoiUI`))))
  (set `/Game/Blueprints/UI/HelpTextUI_BP.helpTextVisibility` "Visible" _hanoiui)
  (`KismetSystemLibrary.Delay` 4.0)
  (set `/Game/Blueprints/UI/HelpTextUI_BP.helpTextVisibility` "Hidden" _hanoiui))

(event `self.PuzzeSolveArea.OnComponentEndOverlap`
  (params (OverlappedComponent :type "PrimitiveComponent Object Reference") (OtherActor :type "Actor Object Reference") (OtherComp :type "PrimitiveComponent Object Reference") (OtherBodyIndex :type Integer))
  ;[1 1 1] Toggle Player Can Solve Puzzle
  (set `self.playerIsInSolveArea` false)
  ;[1 1 1] Toggle Puzzle Help UI
  (set `/Game/Blueprints/UI/HelpTextUI_BP.helpTextVisibility` "Hidden" (`self.HanoiUI`)))

(fn `getCurrDisk`
  (params (value :type Integer))
  (returns (disk :type "/Game/Blueprints/HanoiDisk_BP Object Reference"))
  (for _array_element (`self.DiskActors`)
    (if (== (`/Game/Blueprints/HanoiDisk_BP.diskValue` _array_element) value)
      (set `self.CurrDisk` _array_element)
      (return (`self.CurrDisk`))))
  (return (`self.CurrDisk`)))

(fn `interactWithPeg`
  (params (Peg :type "Array of Integer") (CurrPegID :type Integer))
  (returns (PegOut :type "Array of Integer"))
  (bind _currpeg (`self.CurrPeg`))
  (bind _activedisk (`self.activeDisk`))
  (bind _currpeg_2 (`self.CurrPeg`))
  (bind _isnotempty (`self.isEmptyPeg` _currpeg))
  ;[1 1 1] Pickup from or place disk on current peg
  (set `self.CurrPeg` Peg)
  (set `self.CurrPegID` CurrPegID)
  ;;[0.02144 1 0.3782] Pickup Disk
  (if (`self.isPickup`)
    (if _isnotempty
      (set `self.activeDisk` (`KismetArrayLibrary.Array_Get` _currpeg_2 (`KismetArrayLibrary.Array_LastIndex` _currpeg_2)))
      (set `self.isPickup` false)
      (`KismetArrayLibrary.Array_RemoveItem` (`self.CurrPeg`) (`self.activeDisk`))
      (`|ExecutionSequence`
        (:`then_0`
          ;[1 1 1] Move selected disk up to hover above peg
          (bind _disk (`self.getCurrDisk` (`self.activeDisk`)))
          (`self.K2_AddActorWorldOffset` _disk (`KismetMathLibrary.MakeVector` 0.0 0.0 (- 200.0 (* (+ (`KismetMathLibrary.Conv_IntToDouble` (`KismetArrayLibrary.Array_Length` (`self.CurrPeg`))) 1.0) 20.0))) false false))
        (:`then_1`
          (return (`self.CurrPeg`))))
      (else
        (`AudioComponent.Play` (`self.ErrorSound`) 0.0)
        (return (`self.CurrPeg`))))
    (else
      ;;[0 0.1208 1] Place Disk
      (if _isnotempty
        (if (`self.isLegalMove` _activedisk _currpeg)
          (`KismetArrayLibrary.Array_Add` _currpeg _activedisk :!label _label)
          (set `self.isPickup` true)
          (`|ExecutionSequence`
            (:`then_0`
              _)
            (:`then_1`
              (return (`self.CurrPeg`))))
          (else
            (`AudioComponent.Play` (`self.ErrorSound`) 0.0)
            (return (`self.CurrPeg`))))
        (else
          (goto _label)))
      ;[1 1 1] Move selected disk on to selected pag, stacking with any other disk on peg
      (bind _disk_2 (`self.getCurrDisk` (`self.activeDisk`)))
      (`self.K2_AddActorWorldOffset` _disk_2 (`KismetMathLibrary.MakeVector` (`KismetMathLibrary.Conv_IntToDouble` (* (- (`self.CurrPegID`) (`/Game/Blueprints/HanoiDisk_BP.LastPeg` _disk_2)) -200)) 0.0 (* (- 200.0 (* (`KismetMathLibrary.Conv_IntToDouble` (`KismetArrayLibrary.Array_Length` (`self.CurrPeg`))) 20.0)) -1.0)) false false)
      (set `/Game/Blueprints/HanoiDisk_BP.LastPeg` (`self.CurrPegID`) _disk_2))))

(fn `isEmptyPeg`
  (params (peg :type "Array of Integer"))
  (returns (isNotEmpty :type Boolean))
  (return (> (`KismetArrayLibrary.Array_Length` peg) 0)))

(fn `isGameOver`
  (params (FinalPeg :type "Array of Integer"))
  (returns (GameWon :type Boolean))
  (return (== (`KismetArrayLibrary.Array_Length` FinalPeg) (`self.NUM_DISKS`))))

(fn `isLegalMove`
  (params (disk :type Integer) (targetPeg :type "Array of Integer"))
  (returns (isLegal :type Boolean))
  (return (> (`KismetArrayLibrary.Array_Get` targetPeg (`KismetArrayLibrary.Array_LastIndex` targetPeg)) disk)))

(fn `printGame`
  (`|ExecutionSequence`
    (:`then_0`
      (`KismetSystemLibrary.PrintString` "Printing Peg 1:")
      (for _array_element (`self.Peg1`)
        (`KismetSystemLibrary.PrintString` (`KismetStringLibrary.Conv_IntToString` _array_element) true true (struct :`R` 0.080591 :`G` 1.0 :`B` 0.125712 :`A` 1.0))))
    (:`then_1`
      (`KismetSystemLibrary.PrintString` "Printing Peg 2:")
      (for _array_element_2 (`self.Peg2`)
        (`KismetSystemLibrary.PrintString` (`KismetStringLibrary.Conv_IntToString` _array_element_2) true true (struct :`R` 0.080591 :`G` 1.0 :`B` 0.125712 :`A` 1.0))))
    (:`then_2`
      (`KismetSystemLibrary.PrintString` "Printing Peg 3:")
      (for _array_element_3 (`self.Peg3`)
        (`KismetSystemLibrary.PrintString` (`KismetStringLibrary.Conv_IntToString` _array_element_3) true true (struct :`R` 0.080591 :`G` 1.0 :`B` 0.125712 :`A` 1.0))))))

(fn `UserConstructionScript`)
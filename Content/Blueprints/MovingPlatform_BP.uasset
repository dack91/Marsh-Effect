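; Moving platform Blueprint that slides the Ship2ElevatorPlatform component between a start and end position while it is active.
; Tick sets the timeline play rate from PlatformSpeed and plays the timeline, whose driver lerps the platform's relative location without sweeping.
; Activation is a per-frame IsActive check, marked as a temporary stand-in for fragment-based activation.
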(event `self.ReceiveTick`
  (params (DeltaSeconds :type "Float (single-precision)"))
  ;[1 1 1] TMP: replace with fragment activation
  (if (`self.isActive`)
    ;[1 1 1] Moving Platform
    ;;[1 1 1] Set Platform Speed
    (`TimelineComponent.SetPlayRate` (`self.Timeline_Platform`) (`self.platformSpeed`))
    (bind (_direction _driver) (`Timeline|Timeline_Platform`)
      (:`Update`
        (`SceneComponent.K2_SetRelativeLocation` (`self.ship2_elevator_platform`) (`KismetMathLibrary.VLerp` (`self.startPos`) (`self.endPos`) _driver) false false)))))

(fn `UserConstructionScript`)
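; Engine fragment pickup actor that grants the player the engine fragment when overlapped.
; The first MyPlayer overlap sets HasEngineFragment, plays PickupSuccess, toggles off the fragment's visibility and destroys the actor after a delay so the sound can play.
; BeginPlay caches the player, and Tick polls it to show the pillar light once the player has the navigation fragment.
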(event `self.ReceiveActorBeginOverlap`
  (params (OtherActor :type "Actor Object Reference"))
  ;[1 1 1] Get Player Reference
  (bind _asmy_player (cast `/Game/Blueprints/MyPlayer` OtherActor))
  (set `self.Player1` _asmy_player)
  (if (not (`self.hasBeenPickedUp`))
    (`AudioComponent.Play` (`self.PickupSuccess`) 0.0)
    ;[1 1 1] Update Player Fragment Inventory
    (set `/Game/Blueprints/MyPlayer.hasEngineFragment` true (`self.Player1`))
    ;[1 1 1] Turn off visibility and functionality while sound plays and actor destructs
    (`SceneComponent.ToggleVisibility` (`self.EngineFragment`) false)
    (set `self.hasBeenPickedUp` true)
    (`KismetSystemLibrary.Delay` 2.5)
    (`self.K2_DestroyActor`) ; Destroy Oxygen Fragment, one time use
  ))

(event `self.ReceiveBeginPlay`
  ;[1 1 1] Get player character
  (bind _asmy_player (cast `/Game/Blueprints/MyPlayer` (`GameplayStatics.GetPlayerCharacter` 0)))
  (set `self.Player1` _asmy_player))

(event `self.ReceiveTick`
  (params (DeltaSeconds :type "Float (single-precision)"))
  (if (`/Game/Blueprints/MyPlayer.hasNavigationFragment` (`self.Player1`))
    (`SceneComponent.SetVisibility` (`self.Pilliar_Light`) true false)))

(fn `UserConstructionScript`)
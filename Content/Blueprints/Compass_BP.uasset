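; Compass actor that prints which of eight directions the player character faces when Tab is pressed.
; It enables input for player 0 on BeginPlay, then on each press offsets the character's yaw by half an octant and shifts negative values into a 0-360 range.
; Dividing by 45 and flooring gives an octant index, which a switch maps to a direction enum printed to screen.
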(event `self.ReceiveBeginPlay`
  ;[1 1 1] Enable Player Input
  (`self.EnableInput` (`GameplayStatics.GetPlayerController` 0)))

(event `Key|Tab`
  (params (Key :type "Key Structure" :default "AnyKey"))
  (bind _yaw (.yaw (`KismetMathLibrary.ComposeRotators` (`self.K2_GetActorRotation` (`GameplayStatics.GetPlayerCharacter` 0)) (struct :`Yaw` 22.5))))
  (:`Pressed`
    (switch `int` (`KismetMathLibrary.FFloor` (/ (`KismetMathLibrary.SelectFloat` _yaw (+ _yaw 360.0) (> _yaw 0.0)) 45.0))
      (:`0`
        ;[1 1 1] Compass Enum
        (set `self.DirectionEnum` "NewEnumerator0"))
      (:`1`
        (set `self.DirectionEnum` "NewEnumerator1"))
      (:`2`
        (set `self.DirectionEnum` "NewEnumerator2"))
      (:`3`
        (set `self.DirectionEnum` "NewEnumerator3"))
      (:`4`
        (set `self.DirectionEnum` "NewEnumerator4"))
      (:`5`
        (set `self.DirectionEnum` "NewEnumerator5"))
      (:`6`
        (set `self.DirectionEnum` "NewEnumerator6"))
      (:`7`
        (set `self.DirectionEnum` "NewEnumerator7")))
    ;[1 1 1] Print Direction to Screen
    (`KismetSystemLibrary.PrintString` (`|GetEnumeratorNameAsString` (`self.DirectionEnum`)))))

(fn `UserConstructionScript`)
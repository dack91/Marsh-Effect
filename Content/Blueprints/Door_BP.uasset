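; Door Blueprint that slides two door halves open when something overlaps its box trigger and closes them when the overlap ends.
; A timeline lerps the left and right meshes' relative locations from a shared start to separate end points, and reverses on exit.
; The DoorCanOpen flag gates movement and open/close sounds; when it is false, entering the trigger plays a locked sound instead.
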(event `self.BoxTrigger.OnComponentBeginOverlap`
  (params (OverlappedComponent :type "PrimitiveComponent Object Reference") (OtherActor :type "Actor Object Reference") (OtherComp :type "PrimitiveComponent Object Reference") (OtherBodyIndex :type Integer) (bFromSweep :type Boolean) (SweepResult :type "HitResult Structure (by ref)"))
  ;[1 1 1] Door
  (if (`self.doorCanOpen`)
    (`AudioComponent.Play` (`self.DoorOpenSound`) 0.0)
    (bind (_direction _driver) (`Timeline|Timeline_Door Driver` :!label _label)
      (:`Update`
        (`|ExecutionSequence`
          (:`then_0`
            (`SceneComponent.K2_SetRelativeLocation` (`self.ship2_door_decahedron_L`) (`KismetMathLibrary.VLerp` (`self.DoorStart`) (`self.DoorEndLeft`) _driver) false false))
          (:`then_1`
            (`SceneComponent.K2_SetRelativeLocation` (`self.ship2_door_decahedron_R`) (`KismetMathLibrary.VLerp` (`self.DoorStart`) (`self.DoorEndRight`) _driver) false false)))))
    (else
      (`AudioComponent.Play` (`self.doorLockedSound`) 0.0))))

(event `self.BoxTrigger.OnComponentEndOverlap`
  (params (OverlappedComponent :type "PrimitiveComponent Object Reference") (OtherActor :type "Actor Object Reference") (OtherComp :type "PrimitiveComponent Object Reference") (OtherBodyIndex :type Integer))
  ;[1 1 1] Door
  (if (`self.doorCanOpen`)
    (`AudioComponent.Play` (`self.DoorCloseSound`) 0.0)
    (goto _label :!via `Reverse`)))

(fn `UserConstructionScript`)
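; Simon Says puzzle actor where the player repeats a flashed colour sequence by standing in red, green, blue or yellow boxes and pressing E.
; Entering the outer box rolls four random colours, and Display replays the growing Memory array with lights and sounds through a retriggerable-delay loop.
; Correct presses advance through the stages to a success jingle, while a wrong box triggers error feedback and a new roll.
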(event `self.RedBox (left).OnComponentBeginOverlap`
  (params (OverlappedComponent :type "PrimitiveComponent Object Reference") (OtherActor :type "Actor Object Reference") (OtherComp :type "PrimitiveComponent Object Reference") (OtherBodyIndex :type Integer) (bFromSweep :type Boolean) (SweepResult :type "HitResult Structure (by ref)"))
  ;[1 1 1] Overlaps
  (set `self.InRed` true))

(event `self.GreenBox(midleft).OnComponentBeginOverlap`
  (params (OverlappedComponent :type "PrimitiveComponent Object Reference") (OtherActor :type "Actor Object Reference") (OtherComp :type "PrimitiveComponent Object Reference") (OtherBodyIndex :type Integer) (bFromSweep :type Boolean) (SweepResult :type "HitResult Structure (by ref)"))
  ;[1 1 1] Overlaps
  (set `self.InGreen` true))

(event `self.BlueBox(midright).OnComponentBeginOverlap`
  (params (OverlappedComponent :type "PrimitiveComponent Object Reference") (OtherActor :type "Actor Object Reference") (OtherComp :type "PrimitiveComponent Object Reference") (OtherBodyIndex :type Integer) (bFromSweep :type Boolean) (SweepResult :type "HitResult Structure (by ref)"))
  ;[1 1 1] Overlaps
  (set `self.InBlue` true))

(event `self.YellowBox(right).OnComponentBeginOverlap`
  (params (OverlappedComponent :type "PrimitiveComponent Object Reference") (OtherActor :type "Actor Object Reference") (OtherComp :type "PrimitiveComponent Object Reference") (OtherBodyIndex :type Integer) (bFromSweep :type Boolean) (SweepResult :type "HitResult Structure (by ref)"))
  ;[1 1 1] Overlaps
  (set `self.InYellow` true))

(event `self.OuterBox.OnComponentBeginOverlap`
  (params (OverlappedComponent :type "PrimitiveComponent Object Reference") (OtherActor :type "Actor Object Reference") (OtherComp :type "PrimitiveComponent Object Reference") (OtherBodyIndex :type Integer) (bFromSweep :type Boolean) (SweepResult :type "HitResult Structure (by ref)"))
  ;[1 1 1] Overlaps
  (set `self.InArea` true)
  (`KismetSystemLibrary.PrintString` "Simon Says")
  (`self.Init`))

(event `self.RedBox (left).OnComponentEndOverlap`
  (params (OverlappedComponent :type "PrimitiveComponent Object Reference") (OtherActor :type "Actor Object Reference") (OtherComp :type "PrimitiveComponent Object Reference") (OtherBodyIndex :type Integer))
  ;[1 1 1] Overlaps
  (set `self.InRed` false))

(event `self.GreenBox(midleft).OnComponentEndOverlap`
  (params (OverlappedComponent :type "PrimitiveComponent Object Reference") (OtherActor :type "Actor Object Reference") (OtherComp :type "PrimitiveComponent Object Reference") (OtherBodyIndex :type Integer))
  ;[1 1 1] Overlaps
  (set `self.InGreen` false))

(event `self.BlueBox(midright).OnComponentEndOverlap`
  (params (OverlappedComponent :type "PrimitiveComponent Object Reference") (OtherActor :type "Actor Object Reference") (OtherComp :type "PrimitiveComponent Object Reference") (OtherBodyIndex :type Integer))
  ;[1 1 1] Overlaps
  (set `self.InBlue` false))

(event `self.YellowBox(right).OnComponentEndOverlap`
  (params (OverlappedComponent :type "PrimitiveComponent Object Reference") (OtherActor :type "Actor Object Reference") (OtherComp :type "PrimitiveComponent Object Reference") (OtherBodyIndex :type Integer))
  ;[1 1 1] Overlaps
  (set `self.InYellow` false))

(event `self.OuterBox.OnComponentEndOverlap`
  (params (OverlappedComponent :type "PrimitiveComponent Object Reference") (OtherActor :type "Actor Object Reference") (OtherComp :type "PrimitiveComponent Object Reference") (OtherBodyIndex :type Integer))
  ;[1 1 1] Overlaps
  (set `self.InArea` false)
  (`KismetSystemLibrary.PrintString` "Goodbye")
  (set `self.Stage` 0))

(event `self.ReceiveActorBeginOverlap`
  (params (OtherActor :type "Actor Object Reference"))
  ;[1 1 1] Begin Overlap
  (`self.EnableInput` (`GameplayStatics.GetPlayerController` 0)))

(event `self.ReceiveActorEndOverlap`
  (params (OtherActor :type "Actor Object Reference"))
  ;[1 1 1] Begin Overlap
  (`self.DisableInput` null))

(event `Key|E`
  (params (Key :type "Key Structure" :default "AnyKey"))
  (bind _stage (`self.Stage`))
  (:`Pressed`
    (switch `int` (`KismetArrayLibrary.Array_Get` (`self.Colour`) (`self.LightNumber`))
      (:`0`
        (if (`self.InRed`)
          (if (< (`self.LightNumber`) (`self.Stage`)) :!label _label
            (`/Engine/EditorBlueprintResources/StandardMacros.IncrementInt` (`self.LightNumber`)
              (:`  `
                (`KismetSystemLibrary.PrintString` "LIGHT NUMBER ++")))
            (elif (< _stage 3)
              (`/Engine/EditorBlueprintResources/StandardMacros.IncrementInt` _stage
                (:`  `
                  (`KismetArrayLibrary.Array_Add` (`self.Memory`) (`KismetArrayLibrary.Array_Get` (`self.Colour`) (`self.Stage`)))
                  (`KismetSystemLibrary.PrintString` "STAGE ++")
                  (set `self.LightNumber` 0)
                  (`self.Display`)))
              (else
                (`self.light event` 0 0.0)
                (`KismetSystemLibrary.Delay` 2.0)
                (`self.light event` 1 0.5)
                (`KismetSystemLibrary.Delay` 0.5)
                (`self.light event` 2 0.5)
                (`KismetSystemLibrary.Delay` 0.5)
                (`self.light event` 3 0.5)
                (`KismetSystemLibrary.Delay` 0.5)
                (`AudioComponent.Play` (`self.SuccessAudio`) 0.0))))
          (else
            (if (and (not (or (`self.InRed`) (`self.InGreen`) (`self.InBlue`) (`self.InYellow`))) (`self.InArea`)) :!label _label_2
              (`KismetSystemLibrary.PrintString` "GET CLOSER")
              (else
                (`KismetSystemLibrary.PrintString` "FAIL")
                (`self.Failure`))))))
      (:`1`
        (if (`self.InGreen`)
          (goto _label)
          (else
            (goto _label_2))))
      (:`2`
        (if (`self.InBlue`)
          (goto _label)
          (else
            (goto _label_2))))
      (:`3`
        (if (`self.InYellow`)
          (goto _label)
          (else
            (goto _label_2)))))))

(event `Display`
  (bind _memory (`self.Memory`))
  (bind _item (`KismetArrayLibrary.Array_Get` _memory (`self.int`)))
  ;[1 1 1] Display
  (set `self.int` 0)
  (`self.light event` _item :!label _label_3)
  (`self.audio event` _item)
  (`KismetSystemLibrary.RetriggerableDelay` 1.0)
  (bind _result (`/Engine/EditorBlueprintResources/StandardMacros.IncrementInt` (`self.int`))
    (:`  `
      (if (not (== _result (`KismetArrayLibrary.Array_Length` _memory)))
        (goto _label_3)))))

(event `light event`
  (params (colourevent :type Integer) (delay :type "Float (double-precision)" :default 1.0))
  (bind _redlight (`self.RedLight`))
  (bind _bluelight (`self.BlueLight`))
  (bind _greenlight (`self.GreenLight`))
  (bind _yellowlight (`self.YellowLight`))
  ;[1 1 1] Light Event
  (switch `int` colourevent
    (:`0`
      (`SceneComponent.SetVisibility` _redlight true false)
      (`KismetSystemLibrary.Delay` delay)
      (`SceneComponent.SetVisibility` _redlight false false))
    (:`1`
      (`SceneComponent.SetVisibility` _greenlight true false)
      (`KismetSystemLibrary.Delay` delay)
      (`SceneComponent.SetVisibility` _greenlight false false))
    (:`2`
      (`SceneComponent.SetVisibility` _bluelight true false)
      (`KismetSystemLibrary.Delay` delay)
      (`SceneComponent.SetVisibility` _bluelight false false))
    (:`3`
      (`SceneComponent.SetVisibility` _yellowlight true false)
      (`KismetSystemLibrary.Delay` delay)
      (`SceneComponent.SetVisibility` _yellowlight false false))))

(event `Failure`
  ;[1 1 1] Failure
  (`AudioComponent.Play` (`self.ErrorAudio`) 0.0)
  (`self.reset`)
  (`self.Init`))

(event `Init`
  ;[1 1 1] Init
  (bind _output_get (set `self.Colour` (`|MakeArray` (`KismetMathLibrary.RandomIntegerInRange` 0 3) (`KismetMathLibrary.RandomIntegerInRange` 0 3) (`KismetMathLibrary.RandomIntegerInRange` 0 3) (`KismetMathLibrary.RandomIntegerInRange` 0 3))))
  (`KismetArrayLibrary.Array_Clear` (`self.Memory`))
  (`KismetArrayLibrary.Array_Add` (`self.Memory`) (`KismetArrayLibrary.Array_Get` _output_get))
  (`self.Display`))

(event `reset`
  ;[1 1 1] reset
  (`self.DisableInput` null)
  (set `self.error` true)
  (`self.light event` 0 0.0)
  (`self.light event` 1 0.0)
  (`self.light event` 2 0.0)
  (`self.light event` 3 0.0)
  (`KismetSystemLibrary.Delay` 1.0)
  (`self.light event` 0 0.0)
  (`self.light event` 1 0.0)
  (`self.light event` 2 0.0)
  (`self.light event` 3 0.0)
  (`KismetSystemLibrary.Delay` 1.0)
  (set `self.error` false)
  (`KismetSystemLibrary.Delay` 0.25)
  (`self.EnableInput` null))

(event `audio event`
  (params (colourevent :type Integer))
  ;[1 1 1] audio event
  (switch `int` colourevent
    (:`0`
      (`AudioComponent.Play` (`self.RedAudio`) 0.0))
    (:`1`
      (`AudioComponent.Play` (`self.GreenAudio`) 0.0))
    (:`2`
      (`AudioComponent.Play` (`self.BlueAudio`) 0.0))
    (:`3`
      (`AudioComponent.Play` (`self.YellowAudio`) 0.0))))

(fn `UserConstructionScript`)
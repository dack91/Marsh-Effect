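; A one-time pickup Blueprint for a speeder fragment that the player collects by walking into it.
; On actor overlap with MyPlayer, it plays a pickup sound, hides the EngineFragment component and sets the player's HasSpeederFragment flag.
; A HasBeenPickedUp guard blocks repeat triggers, and a short delay lets the sound play before the actor destroys itself.
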(event `self.ReceiveActorBeginOverlap`
  (params (OtherActor :type "Actor Object Reference"))
  ;[1 1 1] Get Player Reference
  (bind _asmy_player (cast `/Game/Blueprints/MyPlayer` OtherActor))
  (set `self.Player1` _asmy_player)
  (if (not (`self.hasBeenPickedUp`))
    (`AudioComponent.Play` (`self.PickupSuccess`) 0.0)
    ;[1 1 1] Turn off visibility and functionality while sound plays and actor destructs
    (`SceneComponent.ToggleVisibility` (`self.EngineFragment`) false)
    (set `self.hasBeenPickedUp` true)
    (set `/Game/Blueprints/MyPlayer.hasSpeederFragment` true (`self.Player1`))
    (`KismetSystemLibrary.Delay` 2.5)
    ;[1 1 1] Update Player Fragment Inventory
    (`self.K2_DestroyActor`) ; Destroy Oxygen Fragment, one time use
  ))

(fn `UserConstructionScript`)
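; OxygenBonus_BP is a one-time pickup that refills the player's oxygen tank.
; On actor overlap it casts to MyPlayer and adds OxygenBonus to OxygenTank, capping the result at full.
; It then plays the pickup sound, hides the fragment and sets HasBeenPickedUp to block repeat pickups.
; A short delay keeps the actor alive while the sound plays, then it destroys itself.
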(event `self.ReceiveActorBeginOverlap`
  (params (OtherActor :type "Actor Object Reference"))
  (bind _returnvalue (+ (`/Game/Blueprints/MyPlayer.oxygenTank` (`self.Player1`)) (`self.OxygenBonus`)))
  ;[1 1 1] Get Player Reference
  (bind _asmy_player (cast `/Game/Blueprints/MyPlayer` OtherActor))
  (set `self.Player1` _asmy_player)
  (if (not (`self.hasBeenPickedUp`))
    (if (< _returnvalue 1.0)
      ;[1 1 1] Increase Oxygen
      (set `/Game/Blueprints/MyPlayer.oxygenTank` _returnvalue (`self.Player1`))
      (else
        (set `/Game/Blueprints/MyPlayer.oxygenTank` 1.0 (`self.Player1`))))
    (`AudioComponent.Play` (`self.oxygenPickupSound`) 0.0)
    ;[1 1 1] Turn off visibility and functionality while sound plays and actor destructs
    (`SceneComponent.ToggleVisibility` (`self.OxygenFragment`) false)
    (set `self.hasBeenPickedUp` true)
    (`KismetSystemLibrary.Delay` 2.5)
    (`self.K2_DestroyActor`) ; Destroy Oxygen Fragment, one time use
  ))

(fn `UserConstructionScript`)